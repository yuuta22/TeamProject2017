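; Side-scroller enemy that patrols along the Y axis, spinning in yaw every tick, and destroys itself when LifePoint runs out.
; Wall hits set Direction from the hit normal's Y, turning it away from obstacles.
; Sphere overlap drains the player character's LifePoint, while capsule overlap with an item enlarges the enemy.
; Timeline turning, line-trace detection and fire-effect death logic remain unconnected and never run.
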(event OnComponentBeginOverlap(Sphere)
  (params (OverlappedComponent :type Primitive%20Component%20Object%20Reference) (OtherActor :type Actor%20Object%20Reference) (OtherComp :type Primitive%20Component%20Object%20Reference) (OtherBodyIndex :type Integer) (bFromSweep :type Boolean) (SweepResult :type Hit%20Result%20Structure%20%28by%20ref%29))
  (bind _asside_scroller_character (Utilities|Casting|CastToSideScrollerCharacter OtherActor))
  (Variables|/Game/SideScrollerBP/Blueprints/SideScrollerCharacter.SideScrollerCharacter_C|SetLifePoint _asside_scroller_character (- (Variables|/Game/SideScrollerBP/Blueprints/SideScrollerCharacter.SideScrollerCharacter_C|GetLifePoint _asside_scroller_character) 0.1)))

(event OnComponentBeginOverlap(CapsuleComponent)
  (params (OverlappedComponent :type Primitive%20Component%20Object%20Reference) (OtherActor :type Actor%20Object%20Reference) (OtherComp :type Primitive%20Component%20Object%20Reference) (OtherBodyIndex :type Integer) (bFromSweep :type Boolean) (SweepResult :type Hit%20Result%20Structure%20%28by%20ref%29))
  (bind _returnvalue (Transformation|GetActorTransform))
  (bind (_location _rotation _scale) (Math|Transform|BreakTransform _returnvalue))
  (Utilities|Casting|CastToitem OtherActor)
  (Transformation|SetActorTransform (Math|Transform|MakeTransform _location _rotation (+ _scale "0.500000,0.500000,0.500000"))))

(event Custom|turn
  ;[1 1 1] ta-nn
)

(event Collision|EventActorBeginOverlap
  (params (OtherActor :type Actor%20Object%20Reference)))

(event EventTick
  (params (DeltaSeconds :type Float%20%28single-precision%29))
  (bind _returnvalue (Transformation|GetActorRotation))
  (bind (_roll _pitch _yaw) (Math|Rotator|BreakRotator _returnvalue))
  ;[1 1 1] ヨコに動く
  (if (<= (Variables|Default|GetLifePoint) 0.0)
    (Actor|DestroyActor)
    (else
      (Pawn|Input|AddMovementInput "0,0.200000, 0" (Variables|Default|Getdirection) false)
      (Transformation|SetActorRotation (Math|Rotator|MakeRotator _roll _pitch (+ _yaw 1e+02))))))

(event Collision|EventHit
  (params (MyComp :type Primitive%20Component%20Object%20Reference) (Other :type Actor%20Object%20Reference) (OtherComp :type Primitive%20Component%20Object%20Reference) (bSelfMoved :type Boolean) (HitLocation :type Vector :default "0, 0, 0") (HitNormal :type Vector :default "0, 0, 0") (NormalImpulse :type Vector :default "0, 0, 0") (Hit :type Hit%20Result%20Structure%20%28by%20ref%29))
  (bind _y (Math|Vector|BreakVector HitNormal))
  ;[1 1 1] 左右反転
  (if (< _y -0.5)
    (Variables|Default|Setdirection -1.0)
    (elif (> _y 0.5)
      (Variables|Default|Setdirection 1.0))))

(fn ConstructionScript)